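; BP_MMOGame is the MMO game mode, providing server-side helpers for player lookup, groups and clans.
; It loops over the PlayerArray to find characters by name or ID, clear groups and clans, and push group member lists to characters.
; BeginPlay stores the first PlayerStart as respawn point, requests the server address, and retries until it can show a non-dedicated server warning.
; A separate event spawns the chat/group server connection actor.
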(event `ClearGroups`
  ;[1 1 1] Clear groups
  (for _array_element (`GameState.PlayerArray` (`GameplayStatics.GetGameState`))
    (set `/Game/MMO/Blueprints/BP_MMOPlayerCharacter.Group` null (`/Game/MMO/Blueprints/BP_MMOPlayerState.MMOCharacter` (cast `/Game/MMO/Blueprints/BP_MMOPlayerState` _array_element :!pure true))) ; clear
  ))

(event `SendGroupMembers`
  ;[1 1 1] Send Group Members (to the clients)
  (for _array_element (`GameState.PlayerArray` (`GameplayStatics.GetGameState`))
    (bind _mmocharacter (`/Game/MMO/Blueprints/BP_MMOPlayerState.MMOCharacter` (cast `/Game/MMO/Blueprints/BP_MMOPlayerState` _array_element :!pure true)))
    (bind _group (`/Game/MMO/Blueprints/BP_MMOPlayerCharacter.Group` _mmocharacter))
    (`/Engine/EditorBlueprintResources/StandardMacros.IsValid` _group ; if has group
      (:`Is Valid`
        (`/Game/MMO/Blueprints/BP_MMOPlayerCharacter.UpdateGroupMembers` _mmocharacter (`/Game/MMO/Blueprints/Groups/BP_Group.Players` _group)))
      (:`Is Not Valid`
        (`/Game/MMO/Blueprints/BP_MMOPlayerCharacter.UpdateGroupMembers` _mmocharacter (`|MakeArray`))))))

(event `ConnectToChatServer`
  ;[1 1 1] Connect to chat/group server
  (bind _returnvalue (`|SpawnActorFromClass` "/Game/MMO/Blueprints/Chat/BP_ServerChatConnect.BP_ServerChatConnect_C" (`KismetMathLibrary.MakeTransform` (0.0 0.0 0.0)) "Undefined" "OverrideRootScale" null null))
  (set `self.ServerChatConnect` _returnvalue))

(event `self.ReceiveBeginPlay`
  (bind _mmoinstance (`/Game/MMO/Blueprints/BPML_ActorMacroLibrary.MMOInstance`))
  (bind _gamehudwidget (`/Game/MMO/Blueprints/BP_MMOInstance.GameHUDWidget` _mmoinstance))
  ;[1 1 1] Begin play
  (bind _outactors (`GameplayStatics.GetAllActorsOfClass` "/Script/Engine.PlayerStart"))
  (set `self.RespawnPoint` (`self.GetTransform` (`|GetArrayItem` _outactors)))
  (`/Engine/EditorBlueprintResources/StandardMacros.IsValid` _mmoinstance :!label _label
    (:`Is Valid`
      (`/Game/MMO/Blueprints/BP_MMOInstance.GetServerAddress` _mmoinstance)
      (if (and (`KismetSystemLibrary.IsServer`) (not (`KismetSystemLibrary.IsDedicatedServer`)))
        (`/Engine/EditorBlueprintResources/StandardMacros.IsValid` _gamehudwidget :!label _label_2
          (:`Is Valid`
            (`Widget.SetVisibility` (`/Game/MMO/Blueprints/UserInterface/WBP_GameHUD.WarningDedicated` _gamehudwidget) "Visible"))
          (:`Is Not Valid`
            (`KismetSystemLibrary.Delay` 0.2)
            (goto _label_2)))))
    (:`Is Not Valid`
      (`KismetSystemLibrary.Delay` 0.2)
      (goto _label))))

(fn `ClearClans`
  (for _array_element (`GameState.PlayerArray` (`GameplayStatics.GetGameState`))
    (set `/Game/MMO/Blueprints/BP_MMOPlayerCharacter.Clan` "" (`/Game/MMO/Blueprints/BP_MMOPlayerState.MMOCharacter` (cast `/Game/MMO/Blueprints/BP_MMOPlayerState` _array_element :!pure true)))))

(fn `FindPlayer`
  (params (Name :type String))
  (returns (Character :type "/Game/MMO/Blueprints/BP_MMOPlayerCharacter Object Reference"))
  (for _array_element (`GameState.PlayerArray` (`GameplayStatics.GetGameState`))
    (bind _mmocharacter (`/Game/MMO/Blueprints/BP_MMOPlayerState.MMOCharacter` (cast `/Game/MMO/Blueprints/BP_MMOPlayerState` _array_element :!pure true)))
    (if (`KismetStringLibrary.EqualEqual_StrStr` Name (`KismetTextLibrary.Conv_TextToString` (`/Game/MMO/Blueprints/BP_MMOCharacter.Name` _mmocharacter)))
      (return _mmocharacter)))
  (return null))

(fn `FindPlayerById`
  (params (Id :type Integer))
  (returns (Character :type "/Game/MMO/Blueprints/BP_MMOPlayerCharacter Object Reference"))
  (for _array_element (`GameState.PlayerArray` (`GameplayStatics.GetGameState`))
    (bind _asbp_mmoplayer_state (cast `/Game/MMO/Blueprints/BP_MMOPlayerState` _array_element :!pure true))
    (if (== (`/Game/MMO/Blueprints/BP_MMOPlayerState.characterId` _asbp_mmoplayer_state) Id)
      (return (`/Game/MMO/Blueprints/BP_MMOPlayerState.MMOCharacter` _asbp_mmoplayer_state))))
  (return null))

(fn `UserConstructionScript`)