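; BP_NPC is an MMO quest NPC that shows an overhead sign when it can start or end quests for the player.
; RefreshSign shows one sign at most, with the turn-in question mark taking priority over the available-quest exclamation mark.
; Helper functions check local player 0's accepted and completed quests against StartsQuests and EndsQuests, returning the matching quests.
; Completion compares kill and bring tasks against one TaskProgress array, with bring tasks indexed after kill tasks.
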(event `RefreshSign`
  (bind _questendsign (`self.QuestEndSign`))
  (bind _queststartsign (`self.QuestStartSign`))
  ;[0.09093 1 0.3993] Refresh the exclamation/question mark over the NPC's head - there can only be one and question mark has priority
  (bind _true (`self.PlayerCanTurnInQuest`))
  (if _true
    (`SceneComponent.SetHiddenInGame` _questendsign false false)
    (`SceneComponent.SetHiddenInGame` _queststartsign true false)
    (else
      (`SceneComponent.SetHiddenInGame` _questendsign true false)
      (bind _true_2 (`self.PlayerCanStartQuest`))
      (`SceneComponent.SetHiddenInGame` _queststartsign (not _true_2) false))))

(fn `PlayerCanStartQuest`
  (returns (True :type Boolean) (AvailableQuests :type "Array of Quest Object Reference"))
  (locals (Output :type Boolean) (OutputQuests :type "Array of Quest Object Reference"))
  (bind _returnvalue (`GameplayStatics.GetPlayerCharacter` 0))
  (bind _asbp_mmoplayer_character (cast `/Game/MMO/Blueprints/BP_MMOPlayerCharacter` _returnvalue :!pure true))
  (`/Engine/EditorBlueprintResources/StandardMacros.IsValid` _returnvalue
    (:`Is Valid`
      (for _array_element (`self.StartsQuests`)
        (if (not (`KismetArrayLibrary.Array_Contains` (`/Game/MMO/Blueprints/BP_MMOPlayerCharacter.CompletedQuests` _asbp_mmoplayer_character) _array_element))
          (bind _true (`/Game/MMO/Blueprints/BP_MMOPlayerCharacter.HasQuest` _asbp_mmoplayer_character _array_element))
          (if (not _true)
            (set `local.Output` true)
            (`KismetArrayLibrary.Array_Add` (`local.OutputQuests`) _array_element))))
      (return (`local.Output`) (`local.OutputQuests`)))
    (:`Is Not Valid`
      (return false (`|MakeArray` null :!type "Quest Object Reference")))))

(fn `PlayerCanTurnInQuest`
  (returns (True :type Boolean) (TurnableQuests :type "Array of Quest Object Reference"))
  (locals (Output :type Boolean) (QuestsOutput :type "Array of Quest Object Reference"))
  (bind _returnvalue (`GameplayStatics.GetPlayerCharacter` 0))
  (`/Engine/EditorBlueprintResources/StandardMacros.IsValid` _returnvalue
    (:`Is Valid`
      (for _array_element (`/Game/MMO/Blueprints/BP_MMOPlayerCharacter.AcceptedQuests` (cast `/Game/MMO/Blueprints/BP_MMOPlayerCharacter` _returnvalue :!pure true))
        (bind _true (`self.QuestIsCompleted` _array_element))
        (bind _quest (break `/Game/MMO/Quests/Blueprints/FAcceptedQuest` _array_element))
        (if (and (`KismetArrayLibrary.Array_Contains` (`self.EndsQuests`) _quest) _true)
          (set `local.Output` true)
          (`KismetArrayLibrary.Array_Add` (`local.QuestsOutput`) _quest)))
      (return (`local.Output`) (`local.QuestsOutput`)))
    (:`Is Not Valid`
      (return false (`|MakeArray` null :!type "Quest Object Reference")))))

(fn `QuestIsCompleted`
  (params (AcceptedQuest :type "/Game/MMO/Quests/Blueprints/FAcceptedQuest Structure"))
  (returns (True :type Boolean))
  (locals (Output :type Boolean :default true))
  (bind (_quest _taskprogress) (break `/Game/MMO/Quests/Blueprints/FAcceptedQuest` AcceptedQuest))
  (bind _killtasks (`Quest.KillTasks` _quest))
  (for (_array_element _array_index) _killtasks
    (if (> (`.NumberOfKills` (break `QuestTaskKill` _array_element)) (`|GetArrayItem` _taskprogress _array_index))
      (set `local.Output` false :!label _label)))
  (for (_array_element_2 _array_index_2) (`Quest.BringTasks` _quest)
    (if (> (`.AmountToBring` (break `QuestTaskBring` _array_element_2)) (`|GetArrayItem` _taskprogress (+ _array_index_2 (`KismetArrayLibrary.Array_Length` _killtasks))))
      (goto _label)))
  (return (`local.Output`)))

(fn `UserConstructionScript`
  (`parent.UserConstructionScript`))