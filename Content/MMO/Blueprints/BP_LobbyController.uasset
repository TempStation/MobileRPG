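; BP_LobbyController runs the startup logic for the MMO lobby.
; After a short delay on BeginPlay, it ends the loading screen through the MMO game instance, disables on-screen messages and calls the instance's server address lookup.
; If the instance has a network failure flagged, it shows a WBP_NetworkFailure widget with the failure type.
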(event `self.ReceiveBeginPlay`
  (bind _mmoinstance (`/Game/MMO/Blueprints/BPML_ActorMacroLibrary.MMOInstance`))
  (`KismetSystemLibrary.Delay` 1.0)
  (`MyGameInstance.EndLoadingScreen` (`/Game/MMO/Blueprints/BPML_ActorMacroLibrary.MMOInstance`))
  (`KismetSystemLibrary.ExecuteConsoleCommand` "DisableAllScreenMessages" null)
  (`/Game/MMO/Blueprints/BP_MMOInstance.GetServerAddress` _mmoinstance)
  ;[1 1 1] If there was a network failure, display the error message
  (if (`/Game/MMO/Blueprints/BP_MMOInstance.NetworkFailure` _mmoinstance)
    (bind _returnvalue (`|CreateWidget` "/Game/MMO/Blueprints/UserInterface/WBP_NetworkFailure.WBP_NetworkFailure_C" null (`/Game/MMO/Blueprints/BP_MMOInstance.NetworkFailureType` _mmoinstance)))
    (`UserWidget.AddToViewport` _returnvalue 100)
    (`KismetSystemLibrary.PrintString` "display network failure")))

(fn `UserConstructionScript`)